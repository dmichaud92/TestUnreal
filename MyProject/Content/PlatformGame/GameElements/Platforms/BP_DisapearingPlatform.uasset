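; BP_DisapearingPlatform is a platform that endlessly cycles between solid and vanished states.
; After a configurable start delay on BeginPlay, two custom events, ActivateCube and DesactivateCube, call each other through fixed delays to form the loop.
; The mesh briefly turns red before the actor is hidden and loses collision, then returns white, visible and collidable.
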(event `self.ReceiveBeginPlay`
  (`KismetSystemLibrary.Delay` (`self.DurationBeforeStart`))
  (`self.Desactivate Cube`))

(event `Activate Cube`
  ;[1 1 1] Plateform Activation and Desactivation
  (`PrimitiveComponent.SetMaterial` (`self.StaticMeshComponent0`) 0 "/Game/PlatformGame/GameElements/Platforms/M_White.M_White")
  (`self.SetActorHiddenInGame` false)
  (`self.SetActorEnableCollision` true)
  (`KismetSystemLibrary.Delay` 2.0)
  (`self.Desactivate Cube`))

(event `Desactivate Cube`
  (`PrimitiveComponent.SetMaterial` (`self.StaticMeshComponent0`) 0 "/Game/PlatformGame/GameElements/Platforms/M_Red.M_Red")
  (`KismetSystemLibrary.Delay` 0.4)
  (`self.SetActorHiddenInGame` true)
  (`self.SetActorEnableCollision` false)
  (`KismetSystemLibrary.Delay` 2.0)
  (`self.Activate Cube`))

(fn `UserConstructionScript`)